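; BP_SunController is a debug-style controller that rotates a directional light as the sun in the toon shader project.
; Keys 1 and 2 toggle two per-tick rotations, the second reversing direction at pitch limits to swing back and forth.
; Key 0 stops both and restores the starting rotation.
; On BeginPlay it adds a WBP_SunRotation widget, which H shows or hides.
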(event Custom|SwitchDirection
  (Variables|Default|SetRotationSpeed_2 (* (Variables|Default|GetRotationSpeed_2) -1.0)))

(event EventBeginPlay
  (Variables|Default|SetDefaultRotation (Variables|/Script/Engine.SceneComponent|GetRelativeRotation (Variables|Default|GetDirectionalLight)))
  (bind _returnvalue (UserInterface|CreateWidget "/Game/ToonShader/Blueprints/WBP_SunRotation.WBP_SunRotation_C"))
  (bind _output_get (Variables|Default|SetWBP_SunRotation _returnvalue))
  (UserInterface|Viewport|AddtoViewport _output_get 0))

(event EventTick
  (params (DeltaSeconds :type Float%20%28single-precision%29))
  (bind _directionallight (Variables|Default|GetDirectionalLight))
  (bind _relativerotation (Variables|/Script/Engine.SceneComponent|GetRelativeRotation _directionallight))
  (Utilities|FlowControl|Sequence
    (:then_0
      (if (Variables|Default|GetShouldTurn_1)
        (Transformation|AddRelativeRotation (Variables|Default|GetDirectionalLight) (Variables|Default|GetRotationSpeed_1) false false)))
    (:then_1
      (if (Variables|Default|GetShouldTurn_2)
        (if (or (>= (.pitch _relativerotation) 15.0) (<= (.pitch _relativerotation) -7e+01))
          (CallFunction|SwitchDirection)
          (Transformation|AddRelativeRotation (Variables|Default|GetDirectionalLight) (Variables|Default|GetRotationSpeed_2) false false)
          (else
            (Transformation|AddRelativeRotation (Variables|Default|GetDirectionalLight) (Variables|Default|GetRotationSpeed_2) false false)))))))

(event Input|KeyboardEvents|0
  (params (Key :type Key%20Structure :default "None"))
  (:Pressed
    (Transformation|SetRelativeRotation (Variables|Default|GetDirectionalLight) (Variables|Default|GetDefaultRotation) false false)
    (Variables|Default|SetShouldTurn_1 false)
    (Variables|Default|SetShouldTurn_2 false)))

(event Input|KeyboardEvents|H
  (params (Key :type Key%20Structure :default "None"))
  (bind _wbp_sunrotation (Variables|Default|GetWBP_SunRotation))
  (:Pressed
    (if (Variables|Default|GetHideUI)
      (Variables|Default|SetHideUI false)
      (Default|ShowUI _wbp_sunrotation)
      (else
        (Variables|Default|SetHideUI true)
        (Default|HideUI _wbp_sunrotation)))))

(event Input|KeyboardEvents|1
  (params (Key :type Key%20Structure :default "None"))
  (:Pressed
    (if (Variables|Default|GetShouldTurn_1)
      (Variables|Default|SetShouldTurn_1 false)
      (else
        (Variables|Default|SetShouldTurn_1 true)))))

(event Input|KeyboardEvents|2
  (params (Key :type Key%20Structure :default "None"))
  (:Pressed
    (if (Variables|Default|GetShouldTurn_2)
      (Variables|Default|SetShouldTurn_2 false)
      (else
        (Variables|Default|SetShouldTurn_2 true)))))

(fn ConstructionScript)

(fn NewFunction0)