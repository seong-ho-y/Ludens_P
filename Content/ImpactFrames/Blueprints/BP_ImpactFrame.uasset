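; Impact frame actor that flashes stylized full-screen post-process materials as named sequences or single frames.
; ActivateEffect builds dynamic material instances from the styles map, rebuilding only when the style changes.
; Each frame lasts a frame count converted through FrameRate on a timeline, or polls global time dilation until slow motion ends.
; Impact direction, character and target positions, stencil values and a four-tone palette feed each material.
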(event Custom|Wait%20for%20slow%20mo%20end
  (if (>= (Class|GameplayStatics|GetGlobalTimeDilation) 1.0)
    (bind _done (CallFunction|NextFrame))
    (if _done
      (Variables|/Script/Engine.PostProcessComponent|SetBlendWeight (Variables|Default|GetPostProcess) 0.0)
      (Variables|Default|SetFrameIndex 0)
      (else
        (CallFunction|PlaySequence)))
    (else
      (Utilities|FlowControl|DelayUntilNextTick)
      (if (Variables|Default|GetWaitingForSlowMoEnd)
        (CallFunction|WaitforSlowMoEnd)))))

(event Custom|StopSingleFrame
  (Variables|/Script/Engine.PostProcessComponent|SetBlendWeight (Variables|Default|GetPostProcess) 0.0))

(event Custom|ShowSingleFrame
  (params (ImpactFrameMaterial :type Material%20Object%20Reference) (SavedDirectionStart :type Vector) (Direction%20end :type Vector) (HeadLocation :type Vector) (PelvisLocation :type Vector) (TargetLocation :type Vector) (CharacterStencilValue :type Integer) (TargetStencilValue :type Integer) (White :type Linear%20Color%20Structure) (Whitish :type Linear%20Color%20Structure) (Gray :type Linear%20Color%20Structure) (Black :type Linear%20Color%20Structure))
  (Variables|Default|SetSavedDirectionStart SavedDirectionStart)
  (CallFunction|SaveParameters Direction%20end HeadLocation PelvisLocation TargetLocation CharacterStencilValue TargetStencilValue White Whitish Gray Black)
  (bind _returnvalue (Rendering|Material|CreateDynamicMaterialInstance ImpactFrameMaterial "None" "None" :!class /Script/Engine.KismetMaterialLibrary))
  (CallFunction|SetPostProcessMaterial _returnvalue)
  (CallFunction|SetMaterialVariables)
  (Variables|/Script/Engine.PostProcessComponent|SetBlendWeight (Variables|Default|GetPostProcess) 1.0))

(event Custom|SaveDirectionStart
  (params (SavedDirectionStart :type Vector))
  (Variables|Default|SetSavedDirectionStart SavedDirectionStart))

(event Custom|UpdateData
  (params (Direction%20end :type Vector) (HeadLocation :type Vector) (PelvisLocation :type Vector) (TargetLocation :type Vector))
  (Variables|Default|SetImpact%20Direction (Math|Vector|Normalize (- Direction%20end (Variables|Default|GetSavedDirectionStart))))
  (Variables|Default|SetHeadLocation HeadLocation)
  (Variables|Default|SetPelvisLocation PelvisLocation)
  (Variables|Default|SetTargetLocation TargetLocation)
  (CallFunction|SetMaterialVariables))

(event Custom|Play%20sequence
  (if (.lastuntilslowmoends (CallFunction|GetImpactFrameatIndex (Variables|Default|GetCurrentSequence) (Variables|Default|GetFrameIndex)))
    (Variables|Default|SetWaitingForSlowMoEnd true)
    (CallFunction|WaitforSlowMoEnd)
    (else
      (Variables|Default|SetWaitingForSlowMoEnd false)
      (Components|Timeline|SetPlayRate (Variables|Default|GetPlayFrame) (/ 1.0 (/ (Math|Conversions|ToFloat(Integer) (.durationframes (CallFunction|GetImpactFrameatIndex (Variables|Default|GetCurrentSequence) (Variables|Default|GetFrameIndex)))) (Variables|Settings|GetFrameRate))))
      (Timeline|PlayFrame PlayFromStart
        (:Finished
          (bind _done (CallFunction|NextFrame))
          (if _done
            (Variables|/Script/Engine.PostProcessComponent|SetBlendWeight (Variables|Default|GetPostProcess) 0.0)
            (Variables|Default|SetFrameIndex 0)
            (else
              (CallFunction|PlaySequence))))))))

(event Custom|Activate%20Effect
  (params (Name :type Name%20%28by%20ref%29) (FrameRate :type Integer) (Direction%20end :type Vector) (HeadLocation :type Vector) (PelvisLocation :type Vector) (TargetLocation :type Vector) (CharacterStencilValue :type Integer) (TargetStencilValue :type Integer) (White :type Linear%20Color%20Structure) (Whitish :type Linear%20Color%20Structure) (Gray :type Linear%20Color%20Structure) (Black :type Linear%20Color%20Structure))
  (if (Variables|Default|GetEnabled)
    (Variables|Settings|SetFrameRate FrameRate)
    (CallFunction|SaveParameters Direction%20end HeadLocation PelvisLocation TargetLocation CharacterStencilValue TargetStencilValue White Whitish Gray Black)
    (if (!= (Variables|Default|GetLastStyleName) Name)
      (bind _sequence_found (CallFunction|SetImpactFramesSequence Name))
      (if _sequence_found
        (Variables|Default|SetLastStyleName Name :!label _label)
        (CallFunction|SetPostProcessMaterial (Utilities|Array|Get(acopy) (Variables|Default|GetImpactFrameMaterialSequence)))
        (CallFunction|SetMaterialVariables)
        (Variables|/Script/Engine.PostProcessComponent|SetBlendWeight (Variables|Default|GetPostProcess) 1.0)
        (CallFunction|PlaySequence))
      (else
        (goto _label)))))

(event EventBeginPlay
  (|CallParentFunction))

(fn ConstructionScript)

(fn AddIFrametoSequence
  (params (Parent :type Material%20Interface%20Object%20Reference) (Duration%20%28frame%29 :type Integer))
  (bind _returnvalue (Rendering|Material|CreateDynamicMaterialInstance Parent "None" "None" :!class /Script/Engine.KismetMaterialLibrary))
  (Utilities|Array|Add (Variables|Default|GetImpactFrameMaterialSequence) _returnvalue)
  (return _returnvalue))

(fn NextFrame
  (Variables|Default|SetFrameIndex (+ (Variables|Default|GetFrameIndex) 1))
  (if (>= (Variables|Default|GetFrameIndex) (Utilities|Array|Length (CallFunction|GetImpactFrameSequence (Variables|Default|GetCurrentSequence))))
    (return true)
    (else
      (CallFunction|SetPostProcessMaterial (Utilities|Array|Get(acopy) (Variables|Default|GetImpactFrameMaterialSequence) (Variables|Default|GetFrameIndex)))
      (CallFunction|SetMaterialVariables)
      (return false))))

(fn SetMaterialVariables
  (bind _impactframematerial (Variables|Default|GetImpactFrameMaterial))
  (Rendering|Material|SetVectorParameterValue _impactframematerial "Impact location" (Math|Conversions|ToLinearColor(Vector) (Transformation|GetActorLocation)) :!class /Script/Engine.MaterialInstanceDynamic)
  (Rendering|Material|SetVectorParameterValue _impactframematerial "Impact direction" (Math|Conversions|ToLinearColor(Vector) (Variables|Default|GetImpact%20Direction)) :!class /Script/Engine.MaterialInstanceDynamic)
  (Rendering|Material|SetVectorParameterValue _impactframematerial "Main character head" (Math|Conversions|ToLinearColor(Vector) (Variables|Default|GetHeadLocation)) :!class /Script/Engine.MaterialInstanceDynamic)
  (Rendering|Material|SetVectorParameterValue _impactframematerial "Main character pelvis" (Math|Conversions|ToLinearColor(Vector) (Variables|Default|GetPelvisLocation)) :!class /Script/Engine.MaterialInstanceDynamic)
  (Rendering|Material|SetVectorParameterValue _impactframematerial "Target location" (Math|Conversions|ToLinearColor(Vector) (Variables|Default|GetTargetLocation)) :!class /Script/Engine.MaterialInstanceDynamic)
  (Rendering|Material|SetScalarParameterValue _impactframematerial "Main character stencil" (Math|Conversions|ToFloat(Integer) (Variables|Settings|GetCharacterStencilValue)) :!class /Script/Engine.MaterialInstanceDynamic)
  (Rendering|Material|SetScalarParameterValue _impactframematerial "Target stencil" (Math|Conversions|ToFloat(Integer) (Variables|Settings|GetTargetStencilValue)) :!class /Script/Engine.MaterialInstanceDynamic)
  (Rendering|Material|SetVectorParameterValue _impactframematerial "White" (Variables|Settings|GetWhite) :!class /Script/Engine.MaterialInstanceDynamic)
  (Rendering|Material|SetVectorParameterValue _impactframematerial "Black" (Variables|Settings|GetBlack) :!class /Script/Engine.MaterialInstanceDynamic)
  (Rendering|Material|SetVectorParameterValue _impactframematerial "Whitish" (Variables|Settings|GetWhitish) :!class /Script/Engine.MaterialInstanceDynamic)
  (Rendering|Material|SetVectorParameterValue _impactframematerial "Gray" (Variables|Settings|GetGray) :!class /Script/Engine.MaterialInstanceDynamic))

(fn SetPostProcessMaterial
  (params (ImpactFrameMaterial :type Material%20Instance%20Dynamic%20Object%20Reference))
  (bind _output_get (Variables|Default|SetImpactFrameMaterial ImpactFrameMaterial))
  (Variables|/Script/Engine.PostProcessComponent|SetSettings (Variables|Default|GetPostProcess) (Utilities|Struct|MakePostProcessSettings (Utilities|Struct|MakeWeightedBlendables (Utilities|Array|MakeArray (Utilities|Struct|MakeWeightedBlendable 1.0 _output_get))))))

(fn SetImpactFramesSequence
  (params (Sequence%20Name :type Name))
  (bind _impactframestylesmap (Variables|Settings|GetImpactFrameStylesMap))
  (bind (_value _returnvalue) (Utilities|Map|Find _impactframestylesmap Sequence%20Name))
  (bind _sequence (Utilities|Struct|BreakST_ImpactFrameSequence _value))
  (if _returnvalue
    (if (Utilities|Array|IsNotEmpty _sequence)
      (Utilities|Array|Clear (Variables|Default|GetImpactFrameMaterialSequence))
      (for (_array_element _array_index) _sequence
        (Utilities|IsValid (.PostProcessMaterial (Utilities|Struct|BreakST_ImpactFrame _array_element))
          (:Is%20Valid
            (CallFunction|AddIFrametoSequence (.PostProcessMaterial (Utilities|Struct|BreakST_ImpactFrame _array_element)) (.DurationFrames (Utilities|Struct|BreakST_ImpactFrame _array_element))))
          (:Is%20Not%20Valid
            (Development|PrintString (Utilities|String|Append "IMPACT FRAME: THE SEQUENCE " (Utilities|String|ToString(Name) Sequence%20Name) " HAS AN INVALID MATERIAL SET AT INDEX " (Utilities|String|ToString(Integer) _array_index) "! PLEASE CHECK THE \"Impact Frame Styles Map\" VARIABLE IN YOUR BP_ImpactFrame INSTANCE.") true true "(R=1.000000,G=0.000000,B=0.000000,A=1.000000)" 6e+01)
            (return false))))
      (Variables|Default|SetCurrentSequence Sequence%20Name)
      (return true)
      (else
        (Development|PrintString (Utilities|String|Append "IMPACT FRAME: THE SEQUENCE " (Utilities|String|ToString(Name) Sequence%20Name) " IS EMPTY! PLEASE CHECK THE \"Impact Frame Styles Map\" VARIABLE IN YOUR BP_ImpactFrame INSTANCE.") true true "(R=1.000000,G=0.000000,B=0.000000,A=1.000000)" 6e+01)
        (return false)))
    (else
      (Development|PrintString (Utilities|String|Append "IMPACT FRAME: THERE IS NO IMPACT FRAME SEQUENCE REGISTERED AS " (Utilities|String|ToString(Name) Sequence%20Name) "! PLEASE CHECK THE \"Impact Frame Styles Map\" VARIABLE IN YOUR BP_ImpactFrame INSTANCE.") true true "(R=1.000000,G=0.000000,B=0.000000,A=1.000000)" 6e+01)
      (return false))))

(fn GetImpactFrameatIndex
  (params (SequenceName :type Name%20%28by%20ref%29) (Index :type Integer))
  (bind _impactframestylesmap (Variables|Settings|GetImpactFrameStylesMap))
  (bind _value (Utilities|Map|Find _impactframestylesmap SequenceName))
  (bind _sequence (Utilities|Struct|BreakST_ImpactFrameSequence _value))
  (if (< Index (Utilities|Array|Length _sequence))
    (return (Utilities|Array|Get(acopy) _sequence Index))
    (else
      (Development|PrintString "Out of range"))))

(fn GetImpactFrameSequence
  (params (Name :type Name%20%28by%20ref%29))
  (return (Utilities|Struct|BreakST_ImpactFrameSequence (.Value (Utilities|Map|Find (Variables|Settings|GetImpactFrameStylesMap) Name)))))

(fn ToggleActivation
  (params (Enabled :type Boolean))
  (bind _ac_slowmotionmanager (Variables|Default|GetAC_SlowMotionManager))
  (bind _output_get (Variables|Default|SetEnabled Enabled))
  (if _output_get
    (Components|Activation|Activate _ac_slowmotionmanager false)
    (else
      (Components|Activation|Deactivate _ac_slowmotionmanager))))

(fn SaveParameters
  (params (Direction%20end :type Vector) (HeadLocation :type Vector) (PelvisLocation :type Vector) (TargetLocation :type Vector) (CharacterStencilValue :type Integer) (TargetStencilValue :type Integer) (White :type Linear%20Color%20Structure) (Whitish :type Linear%20Color%20Structure) (Gray :type Linear%20Color%20Structure) (Black :type Linear%20Color%20Structure))
  (Variables|Settings|SetWhite White)
  (Variables|Settings|SetWhitish Whitish)
  (Variables|Settings|SetGray Gray)
  (Variables|Settings|SetBlack Black)
  (Variables|Default|SetImpact%20Direction (Math|Vector|Normalize (- Direction%20end (Variables|Default|GetSavedDirectionStart))))
  (Variables|Default|SetHeadLocation HeadLocation)
  (Variables|Default|SetPelvisLocation PelvisLocation)
  (Variables|Default|SetTargetLocation TargetLocation)
  (Variables|Settings|SetCharacterStencilValue CharacterStencilValue)
  (Variables|Settings|SetTargetStencilValue TargetStencilValue))