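; Actor component that drives global slow motion, either as a single timed dilation or as a chain of dilation/duration steps.
; Tick measures real-time delta, zero while paused, so next-tick countdown loops ignore the dilation they apply.
; Single instances optionally restore the previous dilation, while chains reset to 1.0 when finished.
; Starting a single instance cancels any chain; chains can append to a running one or replace it, ending the single instance.
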(event Custom|Slow%20motion%20chain
  (params (SlowMotionData :type Array%20of%20ST%20Slow%20Motion%20Data%20Structures) (AddToExistingChain :type Boolean))
  (if (Components|Activation|IsActive)
    (if (Utilities|Array|IsNotEmpty SlowMotionData)
      (if AddToExistingChain
        (if (Utilities|Array|IsNotEmpty (Variables|Default|GetCurrent%20Slow%20motion%20chain))
          (Utilities|Array|AppendArray (Variables|Default|GetCurrent%20Slow%20motion%20chain) SlowMotionData)
          (else
            (Variables|Default|SetCurrent%20Slow%20motion%20chain SlowMotionData :!label _label)
            (Variables|Default|SetSlomoChainIndex 0)
            (CallFunction|EndSlowMotionInstance)
            (CallFunction|RunSlowMotionChain)))
        (else
          (goto _label))))))

(event Custom|Slow%20motion
  (params (TimeDilation :type Float%20%28single-precision%29) (Duration :type Float%20%28double-precision%29) (RestorePrevious :type Boolean))
  (if (Components|Activation|IsActive)
    (Variables|Default|SetDilationBefore (Class|GameplayStatics|GetGlobalTimeDilation))
    (CallFunction|EndSlowMotionChain)
    (Utilities|Time|SetGlobalTimeDilation TimeDilation)
    (Variables|Default|SetTime%20to%20end%20slow%20motion Duration)
    (Utilities|FlowControl|DelayUntilNextTick :!label _label)
    (if (> (Variables|Default|GetTime%20to%20end%20slow%20motion) 0.0)
      (bind _output_get (Variables|Default|SetTime%20to%20end%20slow%20motion (- (Variables|Default|GetTime%20to%20end%20slow%20motion) (Variables|Default|GetNoDilationDeltaTime))))
      (if (<= _output_get 0.0)
        (if RestorePrevious
          (Utilities|Time|SetGlobalTimeDilation (Variables|Default|GetDilationBefore))
          (else
            (Utilities|Time|SetGlobalTimeDilation 1.0)))
        (else
          (goto _label))))))

(event Custom|EndSlowMotionChain
  (Variables|Default|SetTime%20to%20next%20slomo -1.0)
  (Utilities|Array|Clear (Variables|Default|GetCurrent%20Slow%20motion%20chain))
  (Variables|Default|SetSlomoChainIndex 0))

(event Custom|Run%20slow%20motion%20chain
  (bind _current_slow_motion_chain (Variables|Default|GetCurrent%20Slow%20motion%20chain))
  (bind _slomochainindex (Variables|Default|GetSlomoChainIndex))
  (bind _output (Utilities|Array|Get(acopy) _current_slow_motion_chain _slomochainindex))
  (Utilities|Time|SetGlobalTimeDilation (.dilation _output))
  (Variables|Default|SetTime%20to%20next%20slomo (.duration _output))
  (Utilities|FlowControl|DelayUntilNextTick :!label _label)
  (if (> (Variables|Default|GetTime%20to%20next%20slomo) 0.0)
    (bind _output_get (Variables|Default|SetTime%20to%20next%20slomo (- (Variables|Default|GetTime%20to%20next%20slomo) (Variables|Default|GetNoDilationDeltaTime))))
    (if (<= _output_get 0.0)
      (bind _result (Math|Integer|IncrementInt (Variables|Default|GetSlomoChainIndex))
        (:%20%20
          (if (< _result (Utilities|Array|Length (Variables|Default|GetCurrent%20Slow%20motion%20chain)))
            (CallFunction|RunSlowMotionChain)
            (else
              (Utilities|Time|SetGlobalTimeDilation 1.0)
              (CallFunction|EndSlowMotionChain)))))
      (else
        (goto _label)))))

(event Custom|EndSlowMotionInstance
  (Variables|Default|SetTime%20to%20end%20slow%20motion -1.0))

(event EventTick
  (params (DeltaSeconds :type Float%20%28single-precision%29))
  (bind _returnvalue (Utilities|Time|GetRealTimeSeconds))
  (|CallParentFunction DeltaSeconds)
  (Variables|Default|SetNoDilationDeltaTime (Math|Float|SelectFloat 0.0 (- _returnvalue (Variables|Default|GetPreviousTickTime)) (Game|IsGamePaused)))
  (Variables|Default|SetPreviousTickTime _returnvalue))

(event EventBeginPlay
  (|CallParentFunction)
  (Variables|Default|SetPreviousTickTime (Utilities|Time|GetRealTimeSeconds)))