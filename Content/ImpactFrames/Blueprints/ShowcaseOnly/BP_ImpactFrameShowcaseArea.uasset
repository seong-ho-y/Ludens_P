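; Showcase trigger area that switches the level's BP_ImpactFrame effect on while the DefaultPawn is inside its box.
; Box overlap events, plus an initial overlap check one tick after BeginPlay, identify the pawn by display name and call ToggleActivation.
; ToggleActivation forwards the state to the impact frame actor and starts looping or stops animation on skeletal mesh actors inside the box.
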(event OnComponentBeginOverlap(Box)
  (params (OverlappedComponent :type Primitive%20Component%20Object%20Reference) (OtherActor :type Actor%20Object%20Reference) (OtherComp :type Primitive%20Component%20Object%20Reference) (OtherBodyIndex :type Integer) (bFromSweep :type Boolean) (SweepResult :type Hit%20Result%20Structure%20%28by%20ref%29))
  (if (Utilities|String|Contains (Utilities|GetDisplayName OtherActor) "DefaultPawn")
    (CallFunction|ToggleActivation true)))

(event OnComponentEndOverlap(Box)
  (params (OverlappedComponent :type Primitive%20Component%20Object%20Reference) (OtherActor :type Actor%20Object%20Reference) (OtherComp :type Primitive%20Component%20Object%20Reference) (OtherBodyIndex :type Integer))
  (if (Utilities|String|Contains (Utilities|GetDisplayName OtherActor) "DefaultPawn")
    (CallFunction|ToggleActivation false)))

(event EventBeginPlay
  (bind _returnvalue (Actor|GetActorOfClass "/Game/ImpactFrames/Blueprints/BP_ImpactFrame.BP_ImpactFrame_C"))
  (Variables|Default|SetImpactFrame _returnvalue)
  (Utilities|FlowControl|DelayUntilNextTick)
  (bind _array_element (Utilities|Array|ForEachLoopwithBreak (Collision|GetOverlappingActors (Variables|Default|GetBox) 0 :!class /Script/Engine.PrimitiveComponent))
    (:LoopBody
      (if (Utilities|String|Contains (Utilities|GetDisplayName _array_element) "DefaultPawn")
        (CallFunction|ToggleActivation true)))))

(fn ConstructionScript)

(fn ToggleActivation
  (params (Enabled :type Boolean))
  (Default|ToggleActivation (Variables|Default|GetImpactFrame) Enabled)
  (bind _array_element (Utilities|Array|ForEachLoopwithBreak (Collision|GetOverlappingActors (Variables|Default|GetBox) 0 :!class /Script/Engine.PrimitiveComponent))
    (:LoopBody
      (bind _asskeletal_mesh_actor (Utilities|Casting|CastToSkeletalMeshActor _array_element))
      (if Enabled
        (Audio|Components|Audio|Play (Variables|/Script/Engine.SkeletalMeshActor|GetSkeletalMeshComponent _asskeletal_mesh_actor) true)
        (else
          (Audio|Components|Audio|Stop (Variables|/Script/Engine.SkeletalMeshActor|GetSkeletalMeshComponent _asskeletal_mesh_actor)))))))