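; Showcase actor that previews impact frame materials while a DefaultPawn is inside its trigger box, clearing the frame and UI when it leaves.
; A cycling widget shows the material name, with Next and Previous buttons that step through IFrameList with wraparound.
; Each selection moves the level's BP_ImpactFrame to the main character's impact socket and calls ShowSingleFrame with character and target socket locations, stencil values and tone parameters.
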(event OnComponentBeginOverlap(Box)
  (params (OverlappedComponent :type Primitive%20Component%20Object%20Reference) (OtherActor :type Actor%20Object%20Reference) (OtherComp :type Primitive%20Component%20Object%20Reference) (OtherBodyIndex :type Integer) (bFromSweep :type Boolean) (SweepResult :type Hit%20Result%20Structure%20%28by%20ref%29))
  (if (Utilities|String|Contains (Utilities|GetDisplayName OtherActor) "DefaultPawn")
    (CallFunction|DisplayFrameatCurrentIndex)))

(event OnComponentEndOverlap(Box)
  (params (OverlappedComponent :type Primitive%20Component%20Object%20Reference) (OtherActor :type Actor%20Object%20Reference) (OtherComp :type Primitive%20Component%20Object%20Reference) (OtherBodyIndex :type Integer))
  (if (Utilities|String|Contains (Utilities|GetDisplayName OtherActor) "DefaultPawn")
    (CallFunction|ToggleActivation false)))

(event EventBeginPlay
  (bind _returnvalue (Actor|GetActorOfClass "/Game/ImpactFrames/Blueprints/BP_ImpactFrame.BP_ImpactFrame_C"))
  (Variables|Default|SetImpactFrame _returnvalue)
  (Utilities|FlowControl|DelayUntilNextTick)
  (CallFunction|ToggleActivation false)
  (bind _array_element (Utilities|Array|ForEachLoopwithBreak (Collision|GetOverlappingActors (Variables|Default|GetBox) 0 :!class /Script/Engine.PrimitiveComponent))
    (:LoopBody
      (if (Utilities|String|Contains (Utilities|GetDisplayName _array_element) "DefaultPawn")
        (CallFunction|DisplayFrameatCurrentIndex)))))

(fn ConstructionScript)

(fn ToggleActivation
  (params (Enabled :type Boolean))
  (bind _widget (Variables|Default|GetWidget))
  (bind _maincharacter (Variables|Default|GetMainCharacter))
  (bind _skeletalmeshcomponent (Variables|/Script/Engine.SkeletalMeshActor|GetSkeletalMeshComponent _maincharacter))
  (if Enabled
    (Utilities|FlowControl|Sequence
      (:then_0
        (CallFunction|CreateWidgetifNeeded))
      (:then_1
        (if (not (UserInterface|Viewport|IsinViewport _widget))
          (UserInterface|Viewport|AddtoViewport _widget 0)))
      (:then_2
        (Transformation|SetActorLocation (Variables|Default|GetImpactFrame) (Transformation|GetSocketLocation _skeletalmeshcomponent (Variables|Default|GetImpactLocationSocket)) false false)
        (Default|ShowSingleFrame (Variables|Default|GetImpactFrame) (Variables|Default|GetFrameToVisualize) (Transformation|GetSocketLocation _skeletalmeshcomponent (Variables|Default|GetDirectionStartSocket)) (Transformation|GetSocketLocation _skeletalmeshcomponent (Variables|Default|GetDirectionEndSocket)) (Transformation|GetSocketLocation _skeletalmeshcomponent (Variables|Default|GetHeadSocket)) (Transformation|GetSocketLocation _skeletalmeshcomponent (Variables|Default|GetPelvisSocket)) (Transformation|GetSocketLocation (Variables|/Script/Engine.SkeletalMeshActor|GetSkeletalMeshComponent (Variables|Default|GetTarget)) (Variables|Default|GetTargetSocket)) 1 2 (Variables|Default|GetWhite) (Variables|Default|GetWhitish) (Variables|Default|GetGray) (Variables|Default|GetBlack))))
    (else
      (Default|StopSingleFrame (Variables|Default|GetImpactFrame))
      (Utilities|IsValid (Variables|Default|GetWidget)
        (:Is%20Valid
          (Widget|RemovefromParent (Variables|Default|GetWidget)))))))

(fn PreviousIFrame
  (Math|Integer|DecrementInt (Variables|Default|GetIndex)
    (:%20%20
      (CallFunction|DisplayFrameatCurrentIndex))))

(fn NextIFrame
  (Math|Integer|IncrementInt (Variables|Default|GetIndex)
    (:%20%20
      (CallFunction|DisplayFrameatCurrentIndex))))

(fn DisplayFrameatCurrentIndex
  (CallFunction|CreateWidgetifNeeded)
  (Utilities|FlowControl|Sequence
    (:then_0
      (if (>= (Variables|Default|GetIndex) (Utilities|Array|Length (Variables|Default|GetIFrameList)))
        (Variables|Default|SetIndex 0)
        (elif (< (Variables|Default|GetIndex) 0)
          (Variables|Default|SetIndex (- (Utilities|Array|Length (Variables|Default|GetIFrameList)) 1)))))
    (:then_1
      (bind _output_get (Variables|Default|SetFrameToVisualize (Utilities|Array|Get(acopy) (Variables|Default|GetIFrameList) (Variables|Default|GetIndex))))
      (Rendering|Components|TextRender|SetText (Variables|/Game/ImpactFrames/Blueprints/ShowcaseOnly/WD_CycleImpactFrames.WD_CycleImpactFrames_C|GetMaterialname (Variables|Default|GetWidget)) (Utilities|Text|ToText(String) (Utilities|GetDisplayName _output_get)))
      (CallFunction|ToggleActivation true))))

(fn CreateWidgetifNeeded
  (Utilities|IsValid (Variables|Default|GetWidget)
    (:Is%20Not%20Valid
      (bind _returnvalue (UserInterface|CreateWidget "/Game/ImpactFrames/Blueprints/ShowcaseOnly/WD_CycleImpactFrames.WD_CycleImpactFrames_C" (Game|GetPlayerController 0)))
      (bind _output_get (Variables|Default|SetWidget _returnvalue))
      (EventDispatchers|BindEventtoOnPressed (Variables|/Game/ImpactFrames/Blueprints/ShowcaseOnly/WD_CycleImpactFrames.WD_CycleImpactFrames_C|GetButtonNext _output_get) (EventDispatchers|CreateEvent :!event NextIFrame))
      (EventDispatchers|BindEventtoOnPressed (Variables|/Game/ImpactFrames/Blueprints/ShowcaseOnly/WD_CycleImpactFrames.WD_CycleImpactFrames_C|GetButtonPrevious _output_get) (EventDispatchers|CreateEvent :!event PreviousIFrame)))))